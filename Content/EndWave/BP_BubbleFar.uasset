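; BP_BubbleFar is an effect actor that shows a Niagara effect, likely distant bubbles, when a wave ends.
; On BeginPlay it casts the game mode to BP_FirstPersonGameMode and binds to its EndWave dispatcher.
; The EndWave event activates the Niagara component and deactivates it after a five-second delay.
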(event Custom|EndWave
  (Components|Activation|Activate (Variables|Default|GetNiagara) false)
  (Utilities|FlowControl|Delay 5.0)
  (Components|Activation|Deactivate (Variables|Default|GetNiagara)))

(event EventBeginPlay
  (bind _asbp_first_person_game_mode (Utilities|Casting|CastToBP_FirstPersonGameMode (Game|GetGameMode)))
  (bind _output_get (Variables|Default|SetAs%20BP%20First%20Person%20Game%20Mode _asbp_first_person_game_mode))
  (EventDispatchers|BindEventtoEndWave _output_get (EventDispatchers|CreateEvent :!event Custom|EndWave)))

(event Collision|EventActorBeginOverlap
  (params (OtherActor :type Actor%20Object%20Reference)))

(event EventTick
  (params (DeltaSeconds :type Float%20%28single-precision%29)))

(fn ConstructionScript)