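; BP_SoundManager is an actor that plays the game's music and wave transition sounds.
; On BeginPlay it binds to BP_FirstPersonGameMode's wave start and end events and the menu manager's music launch event, then plays a depth-change sound.
; The menu event spawns the 2D music and stores its reference.
; Wave events play one-shot cues and adjust that music's volume, lowering it between waves and raising it during them.
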(event Custom|EndWave
  (Audio|PlaySound2D "/Game/Sound/SoundWave/W_ChangeDepth.W_ChangeDepth" 1.0 1.0 0.0 0 0)
  (Audio|Components|Audio|SetVolumeMultiplier (Variables|Default|GetMusiqueRef) 0.2 :!class /Script/Engine.AudioComponent))

(event Custom|StartWave
  (Audio|PlaySound2D "/Game/Sound/SoundWave/W_Death.W_Death" 1.0 1.0 0.0 0 0)
  (Audio|Components|Audio|SetVolumeMultiplier (Variables|Default|GetMusiqueRef) 0.5 :!class /Script/Engine.AudioComponent))

(event Custom|PlayMusique
  (bind _returnvalue (Audio|SpawnSound2D "/Game/Sound/SoundCue/C_Musique.C_Musique" 0.5 1.0 0.0 0))
  (Variables|Default|SetMusiqueRef _returnvalue))

(event EventBeginPlay
  (bind _asbp_first_person_game_mode (Utilities|Casting|CastToBP_FirstPersonGameMode (Game|GetGameMode)))
  (bind _output_get (Variables|Default|SetAs%20BP%20First%20Person%20Game%20Mode _asbp_first_person_game_mode))
  (EventDispatchers|BindEventtoEndWave _output_get (delegate Custom|EndWave))
  (EventDispatchers|BindEventtoStartWaving _output_get (delegate Custom|StartWave))
  (EventDispatchers|BindEventtoLaucheMusique (Variables|Default|GetMenuManagerRef) (delegate Custom|PlayMusique))
  (Audio|PlaySound2D "/Game/Sound/SoundWave/W_ChangeDepth.W_ChangeDepth" 1.0 1.0 0.0 0 0))

(event Collision|EventActorBeginOverlap
  (params (OtherActor :type Actor%20Object%20Reference)))

(event EventTick
  (params (DeltaSeconds :type Float%20%28single-precision%29)))

(fn ConstructionScript)