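; BP_RefLoc is a reference-location actor that queues enemies, spawns them at its SpawnPoint and can be flagged as a taken seat.
; On BeginPlay it registers in BP_FirstPersonGameMode's RefLocList and starts a looping timer with a randomized interval based on TimeToSpawn.
; AddEnemyToSpawn fills the queue.
; Spawn debug-prints the first entry's drink demands, passes its wants to the new enemy, links it back here and dequeues it.
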(event Custom|Spawn
  (bind _enemylist1 (Variables|Default|GetEnemyList1))
  (bind _spawnpoint (Variables|Default|GetSpawnPoint))
  (bind _output (Utilities|Array|Get(acopy) _enemylist1))
  (bind (_enemy _want) (Utilities|Struct|BreakEnemy _output))
  (Utilities|IsValid _spawnpoint
    (:Is%20Valid
      (if (not (Utilities|Array|IsEmpty _enemylist1))
        (CallFunction|Test)
        (bind _returnvalue (Game|SpawnActorfromClass _enemy (Math|Transform|MakeTransform (Transformation|GetWorldLocation (Variables|/Game/Enemy/BP_SpawnPoint.BP_SpawnPoint_C|GetDefaultSceneRoot _spawnpoint)) "0, 0, 0" "1.000000,1.000000,1.000000") "Undefined" "MultiplyWithRoot" 0 _want 0))
        (Utilities|IsValid _returnvalue
          (:Is%20Valid
            (Variables|/Game/Enemy/BP_Enemy.BP_Enemy_C|SetRefLoc _returnvalue self)
            (Utilities|Array|RemoveIndex (Variables|Default|GetEnemyList1))))))))

(event Custom|Test
  (for _array_element (Utilities|Struct|BreakMultiDemand (.Want (Utilities|Struct|BreakEnemy (Utilities|Array|Get(acopy) (Variables|Default|GetEnemyList1)))))
    (for _array_element_2 (.Drinks (Utilities|Struct|BreakDemand _array_element))
      (Development|PrintString (Utilities|String|EnumtoString _array_element_2) true true "(R=0.000000,G=0.660000,B=1.000000,A=1.000000)" 1.5e+02))))

(event EventBeginPlay
  (bind _timetospawn (Variables|Default|GetTimeToSpawn))
  (bind _asbp_first_person_game_mode (Utilities|Casting|CastToBP_FirstPersonGameMode (Game|GetGameMode)))
  (bind _output_get (Variables|Default|SetAs%20BP%20First%20Person%20Game%20Mode _asbp_first_person_game_mode))
  (Utilities|Array|Add (Variables|/Game/FirstPerson/Blueprints/BP_FirstPersonGameMode.BP_FirstPersonGameMode_C|GetRefLoc_List _output_get) self)
  (Utilities|Time|SetTimerbyEvent (EventDispatchers|CreateEvent :!event Custom|Spawn) (Math|Random|RandomFloatinRange (+ _timetospawn 0.5) (+ _timetospawn 2.5)) true))

(event Collision|EventActorBeginOverlap
  (params (OtherActor :type Actor%20Object%20Reference)))

(event EventTick
  (params (DeltaSeconds :type Float%20%28single-precision%29)))

(event EventSetSitTaken
  (Variables|Default|SetTaken? true))

(fn ConstructionScript)

(fn AddEnemytoSpawn
  (params (Enemy :type Enemy%20Structure) (TimeToSpawn :type Float%20%28double-precision%29))
  (Utilities|Array|Add (Variables|Default|GetEnemyList1) Enemy)
  (Variables|Default|SetTimeToSpawn TimeToSpawn))