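; Drink-demanding customer enemy that walks to a chair, raises player HUD stress while seated and leaves when satisfied.
; A camera-facing plane swaps materials by state, with widgets showing its demand and an indicator.
; A forward trace detects other AI or free chairs to stop or sit.
; DrinkHit removes matching drink and fill pairs, plays timeline-driven reactions, then destroys the emptied enemy and ends the wave when none remain.
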(event OnComponentBeginOverlap(CapsuleComponent)
  (params (OverlappedComponent :type Primitive%20Component%20Object%20Reference) (OtherActor :type Actor%20Object%20Reference) (OtherComp :type Primitive%20Component%20Object%20Reference) (OtherBodyIndex :type Integer) (bFromSweep :type Boolean) (SweepResult :type Hit%20Result%20Structure%20%28by%20ref%29))
  (if (== OtherActor (Variables|Movement|GetRefLoc))
    _))

(event OnComponentEndOverlap(CapsuleComponent)
  (params (OverlappedComponent :type Primitive%20Component%20Object%20Reference) (OtherActor :type Actor%20Object%20Reference) (OtherComp :type Primitive%20Component%20Object%20Reference) (OtherBodyIndex :type Integer))
  (if (== OtherActor (Variables|Movement|GetRefLoc))
    _))

(event Custom|StressPhase
  ;[0.15 0.15 0.15 0.5] Stress
  (bind _returnvalue (Utilities|Time|SetTimerbyEvent (EventDispatchers|CreateEvent :!event Custom|Stress) 1.5 true))
  (Variables|Default|SetTimerStress _returnvalue))

(event Custom|Stress
  ;[0.15 0.15 0.15 0.5] Stress
  (Variables|Default|SetStressValue (Math|Integer|Clamp(Integer) (+ (Variables|Default|GetStressValue) 1) 0 20))
  (if (> (Variables|Default|GetStressValue) 5)
    (if (> (Variables|Default|GetStressValue) 8)
      (if (> (Variables|Default|GetStressValue) 12)
        _))))

(event Custom|Stop
  (Components|Movement|StopMovementImmediately (Variables|Character|GetCharacterMovement))
  (Variables|Movement|SetMustStop? true))

(event Custom|Check
  (bind _capsulecomponent (Variables|Collision|GetCapsuleComponent))
  (bind _returnvalue (Transformation|GetWorldLocation _capsulecomponent))
  ;[0.15 0.15 0.15 0.5] Check Si touche ou non la chaise ou un autre ennemis
  (bind (_outhit _returnvalue_2) (Collision|LineTraceByChannel _returnvalue (+ _returnvalue (* (Math|Vector|GetForwardVector (Variables|Default|GetArrow1)) 45.0)) "TraceTypeQuery1" false 0 "ForDuration"))
  (if _returnvalue_2
    (if (Actor|ActorHasTag (.HitActor (Collision|BreakHitResult _outhit)) "AI")
      (Variables|Movement|SetMustStop? true)
      (CallFunction|StressPhase)
      (Components|Movement|StopMovementImmediately (Variables|Character|GetCharacterMovement))
      (elif (Utilities|DoesObjectImplementInterface (.HitActor (Collision|BreakHitResult _outhit)) "/Game/Enemy/BPI_Chair.BPI_Chair_C")
        (bind _asbp_ref_loc (Utilities|Casting|CastToBP_RefLoc (.HitActor (Collision|BreakHitResult _outhit))))
        (bind _output_get (Variables|Default|SetAs%20BP%20Ref%20Loc_0 _asbp_ref_loc))
        (if (Variables|/Game/Enemy/BP_RefLoc.BP_RefLoc_C|GetTaken? _output_get)
          (Development|PrintString "Hello")
          (else
            (Utilities|FlowControl|DoOnce false
              (:Completed
                (Class|BPIChair|SetSitTaken(Message) (.HitActor (Collision|BreakHitResult _outhit)))
                (Variables|Movement|SetMustStop? true)
                (CallFunction|SitDown)))))
        (else
          (Variables|Movement|SetMustStop? false)
          (Utilities|Time|ClearandInvalidateTimerbyHandle (Variables|Default|GetTimerStress)))))
    (else
      (Variables|Movement|SetMustStop? false))))

(event Custom|SitDown
  ;[0.15 0.15 0.15 0.5] SitDownEvent
  (Variables|Default|SetIsSit true)
  (Rendering|Material|SetMaterial (Variables|Default|GetPlane) 0 (Variables|Default|GetMAngry))
  (Utilities|Time|SetTimerbyEvent (delegate Custom|Sound) 1.5 true)
  (bind _returnvalue (Utilities|Time|SetTimerbyEvent (EventDispatchers|CreateEvent :!event Custom|SitDownStuff) 0.1 true))
  (Variables|Default|SetTimerStress _returnvalue)
  (Development|PrintString "j'ysusi"))

(event Custom|SitDownStuff
  (bind _playerref (Variables|Default|GetPlayerRef))
  (bind _hud (Variables|/Game/FirstPerson/Blueprints/BP_FirstPersonCharacter.BP_FirstPersonCharacter_C|GetHUD _playerref))
  ;[0.15 0.15 0.15 0.5] SitDownEvent
  (Variables|/Game/Widgets/WBP_HUD.WBP_HUD_C|SetTargetStress _hud (+ (Variables|/Game/Widgets/WBP_HUD.WBP_HUD_C|GetTargetStress _hud) 0.001)))

(event Custom|Sound
  (Audio|PlaySoundatLocation "/Game/Sound/SoundCue/C_EnnemieAttack.C_EnnemieAttack" (Transformation|GetActorLocation) "0, 0, 0" 0.2 1.0 0.0 0 0 0 0))

(event EventBeginPlay
  (Audio|PlaySoundatLocation "/Game/Sound/SoundWave/SpawnEnnemie/C_SpawnEnnemie.C_SpawnEnnemie" (Transformation|GetActorLocation) "0, 0, 0" 0.2 1.0 0.0 0 0 0 0)
  (Utilities|FlowControl|Sequence
    (:then_0
      (bind _asbp_first_person_game_mode (Utilities|Casting|CastToBP_FirstPersonGameMode (Game|GetGameMode)))
      (Variables|Default|SetAs%20BP%20First%20Person%20Game%20Mode _asbp_first_person_game_mode)
      (Utilities|Time|SetTimerbyEvent (EventDispatchers|CreateEvent :!event Custom|Check) 0.2 true)
      (Utilities|Array|Add (Variables|/Game/FirstPerson/Blueprints/BP_FirstPersonGameMode.BP_FirstPersonGameMode_C|GetEnemyList (Variables|Default|GetAs%20BP%20First%20Person%20Game%20Mode)) self)
      (Utilities|FlowControl|Delay 1.0)
      (EventDispatchers|BindEventtoStop (Variables|Movement|GetRefLoc) (delegate Custom|Stop)))
    (:then_1
      (bind _asbp_first_person_character (Utilities|Casting|CastToBP_FirstPersonCharacter (Game|Player|GetPlayerPawn 0)))
      (Variables|Default|SetPlayerRef _asbp_first_person_character)
      (bind _hud (Variables|/Game/FirstPerson/Blueprints/BP_FirstPersonCharacter.BP_FirstPersonCharacter_C|GetHUD _asbp_first_person_character :!label _label)
        (:then
          (bind _returnvalue (UserInterface|CreateWidget "/Game/Widgets/WBP_Indicator.WBP_Indicator_C" 0 self _asbp_first_person_character))
          (Variables|Default|SetSkyrim%20bitch _returnvalue)
          (Widget|Panel|AddChild (Variables|/Game/Widgets/WBP_HUD.WBP_HUD_C|GetIndicatorsPanel _hud) _returnvalue))
        (:else
          (Utilities|FlowControl|DelayUntilNextTick)
          (goto _label))))
    (:then_2
      (bind _returnvalue_2 (UserInterface|CreateWidget "/Game/Widgets/WBP_Wants.WBP_Wants_C" 0 (Utilities|Array|Get(acopy) (Utilities|Struct|BreakMultiDemand (Variables|Default|GetWants)))))
      (bind _output_get (Variables|Default|SetWantsWidget _returnvalue_2))
      (UserInterface|SetWidget (Variables|Default|GetWidget) _output_get))
    (:then_3
      (Rendering|Material|SetMaterial (Variables|Default|GetPlane) 0 (Variables|Default|GetMWalk)))))

(event EventTick
  (params (DeltaSeconds :type Float%20%28single-precision%29))
  (bind _refloc (Variables|Movement|GetRefLoc))
  (bind _capsulecomponent (Variables|Collision|GetCapsuleComponent))
  (bind _returnvalue (Transformation|GetWorldLocation _capsulecomponent))
  (bind _arrow (Variables|/Game/Enemy/BP_RefLoc.BP_RefLoc_C|GetArrow _refloc))
  (bind _returnvalue_2 (Transformation|GetWorldLocation _arrow))
  ;[0.15 0.15 0.15 0.5] Movement et look
  (Utilities|FlowControl|Sequence
    (:then_0
      (if (not (Variables|Movement|GetMustStop?))
        (if (AI|Components|NavMovement|IsMovingonGround (Variables|Character|GetCharacterMovement))
          (if (Variables|Default|GetCanMove)
            (Pawn|Input|AddMovementInput (- _returnvalue_2 _returnvalue) 1.0 false)
            (Transformation|SetActorRotation (Math|Rotator|MakeRotator 0.0 0.0 (.yaw (Math|Rotator|FindLookatRotation _returnvalue _returnvalue_2))))))))
    (:then_1
      (Transformation|SetWorldRotation (Variables|Default|GetPlane) (Class|KismetMathLibrary|MakeRotfromYZ (* (Transformation|GetActorUpVector) -1.0) (Math|Vector|Normalize (- (Transformation|GetWorldLocation (Variables|/Game/FirstPerson/Blueprints/BP_FirstPersonCharacter.BP_FirstPersonCharacter_C|GetFirstPersonCamera (Variables|Default|GetPlayerRef))) (Transformation|GetActorLocation)))) false false))))

(event EventDrinkHit
  (params (Drink :type DrinkEnum%20Enum :default "NewEnumerator0") (Fill :type Float%20%28double-precision%29))
  (bind _plane (Variables|Default|GetPlane))
  (bind _as_bp_ref_loc_0 (Variables|Default|GetAs%20BP%20Ref%20Loc_0))
  (bind _wants (Variables|Default|GetWants))
  (bind _output (Utilities|Array|Get(acopy) (.demands _wants)))
  (bind _output_2 (Utilities|Array|Get(acopy) (.demands _wants)))
  ;[0.15 0.15 0.15 0.5] Hit
  (bind _index (Utilities|FlowControl|ForLoopwithBreak 0 (Utilities|Array|LastIndex (.drinks _output)) :!label _label)
    (:LoopBody
      (if (and (Utilities|Enum|Equal(Enum) (Utilities|Array|Get(acopy) (.drinks _output) _index) Drink) (Math|Float|NearlyEqual(Float) (Utilities|Array|Get(acopy) (.fill _output) _index) Fill 0.1))
        (Utilities|FlowControl|Sequence
          (:then_0
            (Utilities|Array|RemoveIndex (.drinks _output_2) _index)
            (Utilities|Array|RemoveIndex (.fill _output_2) _index)
            (if (== (Utilities|Array|Length (.drinks _output_2)) 0)
              (Variables|Default|SetCanMove false)
              (bind _returnvalue (Rendering|Material|CreateDynamicMaterialInstance (Variables|Default|GetMHappy) "None" "None" :!class /Script/Engine.KismetMaterialLibrary))
              (bind _output_get (Variables|Default|SetDMIHit _returnvalue))
              (Rendering|Material|SetMaterial _plane 0 _output_get)
              (Audio|PlaySoundatLocation "/Game/Sound/SoundCue/C_Hit.C_Hit" (Transformation|GetActorLocation) "0, 0, 0" 1.0 1.0 0.0 0 0 0 0)
              (bind _alpha (Timeline|KilledByHappiness PlayFromStart)
                (:Update
                  (Rendering|Material|SetScalarParameterValue (Variables|Default|GetDMIHit) "Percent" (Math|Float|Lerp 1.0 0.0 (Math|Float|Power _alpha 2.0)) :!class /Script/Engine.MaterialInstanceDynamic))
                (:Finished
                  (Widget|RemovefromParent (Variables|Default|GetSkyrim%20bitch))
                  (Utilities|IsValid _as_bp_ref_loc_0
                    (:Is%20Valid
                      (Variables|/Game/Enemy/BP_RefLoc.BP_RefLoc_C|SetTaken? _as_bp_ref_loc_0 false))
                    (:Is%20Not%20Valid
                      _))
                  (Utilities|Array|RemoveItem (Variables|/Game/FirstPerson/Blueprints/BP_FirstPersonGameMode.BP_FirstPersonGameMode_C|GetEnemyList (Variables|Default|GetAs%20BP%20First%20Person%20Game%20Mode)) self)
                  (if (Utilities|Array|IsEmpty (Variables|/Game/FirstPerson/Blueprints/BP_FirstPersonGameMode.BP_FirstPersonGameMode_C|GetEnemyList (Variables|Default|GetAs%20BP%20First%20Person%20Game%20Mode)))
                    (Default|CallEndWave (Variables|Default|GetAs%20BP%20First%20Person%20Game%20Mode))
                    (Development|PrintString "EndWave")
                    (else
                      (Utilities|FlowControl|Delay 0.005)))
                  (Actor|DestroyActor)))
              (else
                (Variables|Default|SetCanMove false)
                (bind _returnvalue_2 (Rendering|Material|CreateDynamicMaterialInstance (Variables|Default|GetMHit) "None" "None" :!class /Script/Engine.KismetMaterialLibrary))
                (bind _output_get_2 (Variables|Default|SetDMIHit _returnvalue_2))
                (Rendering|Material|SetMaterial _plane 0 _output_get_2)
                (Audio|PlaySoundatLocation "/Game/Sound/SoundCue/C_Hit.C_Hit" (Transformation|GetActorLocation) "0, 0, 0" 1.0 1.0 0.0 0 0 0 0)
                (bind _alpha_2 (Timeline|Hit PlayFromStart)
                  (:Update
                    (Rendering|Material|SetScalarParameterValue (Variables|Default|GetDMIHit) "Goomba" (Math|Float|Lerp 0.0 0.5 _alpha_2) :!class /Script/Engine.MaterialInstanceDynamic))
                  (:Finished
                    (Variables|Default|SetCanMove true)
                    (Rendering|Material|SetMaterial (Variables|Default|GetPlane) 0 (select (Variables|Default|GetIsSit) (Variables|Default|GetMAngry) (Variables|Default|GetMWalk))))))))
          (:then_1
            (goto _label Break)))))
    (:Completed
      (Default|LoadDemand (Variables|Default|GetWantsWidget) (Utilities|Array|Get(acopy) (.demands (Variables|Default|GetWants)))))))

(fn ConstructionScript)