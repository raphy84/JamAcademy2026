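; Enemy spawn point that creates an enemy from a queued list at a referenced SpawnPoint's location, framed by a Niagara effect.
; Spawn starts the effect, waits, spawns the first EnemyList1 entry with its Want value, then waits and stops the effect.
; Nothing live here calls Spawn; the looping timer, list add/removal and difficulty-curve experiments are disconnected, so Spawn never advances the list.
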(event Custom|Spawn
  (bind _enemylist1 (Variables|Default|GetEnemyList1))
  (bind _spawnpoint (Variables|Default|GetSpawnPoint))
  (bind _output (Utilities|Array|Get(acopy) _enemylist1))
  (bind (_enemy _want) (Utilities|Struct|BreakEnemy _output))
  (Utilities|IsValid _spawnpoint
    (:Is%20Valid
      (if (not (Utilities|Array|IsEmpty _enemylist1))
        (Development|PrintString (Utilities|String|ToString(Float) (Variables|Default|GetTimeToSpawn)))
        (Components|Activation|Activate (Variables|Default|GetNiagara) false)
        (Utilities|FlowControl|Delay 1.0)
        (Game|SpawnActorfromClass _enemy (Math|Transform|MakeTransform (Transformation|GetWorldLocation (Variables|BP_SpawnPoint_C|GetDefaultSceneRoot _spawnpoint)) "0, 0, 0" "1.000000,1.000000,1.000000") "Undefined" "MultiplyWithRoot" 0 _want 0)
        (Utilities|FlowControl|Delay 1.0)
        (Components|Activation|Deactivate (Variables|Default|GetNiagara))))))

(event Custom|CustomEvent)

(event Custom|CustomEvent_1)

(event Collision|EventActorBeginOverlap
  (params (OtherActor :type Actor%20Object%20Reference)))

(event EventTick
  (params (DeltaSeconds :type Float%20%28single-precision%29)))

(event EventBeginPlay)

(fn ConstructionScript)