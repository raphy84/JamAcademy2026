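; Glass spawner actor that keeps a three-slot rack stocked with BP_Glass actors, spawning the first on BeginPlay.
; Each new glass slides with a timeline-driven tilt to the next free slot, collision off until arrival, then a 10-second timer spawns another unless full.
; TakeShop removes the given glass, slides those behind it forward with a similar tilt, then restarts the spawn timer.
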(event Custom|NewLevel)

(event Custom|SpawnShop
  (bind _returnvalue (Game|SpawnActorfromClass "/Game/Blueprint/BP_Glass.BP_Glass_C" (Math|Transform|MakeTransform (Transformation|GetWorldLocation (Variables|Default|GetSpawnPoint)) "0, 0, 0" "1.000000,1.000000,1.000000") "AlwaysSpawn" "MultiplyWithRoot" 0 0))
  (Collision|SetActorEnableCollision _returnvalue false)
  (Utilities|Array|AddUnique (Variables|Default|GetGlassArray) _returnvalue)
  (Variables|/Game/Blueprint/BP_Glass.BP_Glass_C|SetSpawnerRef _returnvalue self)
  (bind (_direction _alpha _angle) (Timeline|Timeline PlayFromStart)
    (:Update
      (Transformation|SetActorLocation _returnvalue (Math|Vector|Lerp(Vector) (Transformation|GetWorldLocation (Variables|Default|GetSpawnPoint)) (Utilities|Select :Index (Variables|Default|GetRackNum) :Option%200 (Transformation|GetWorldLocation (Variables|Default|GetSpawnPoint1)) :Option%201 (Transformation|GetWorldLocation (Variables|Default|GetSpawnPoint2)) :Option%202 (Transformation|GetWorldLocation (Variables|Default|GetSpawnPoint3))) _alpha) false false)
      (Transformation|SetActorRotation _returnvalue (Math|Rotator|MakeRotfromZX (Math|Vector|RotateVectorAroundAxis "0.000000,0.000000,1.000000" (* _angle 2e+01) (Transformation|GetActorRightVector)) (Transformation|GetActorForwardVector _returnvalue))))
    (:Finished
      (Collision|SetActorEnableCollision _returnvalue true)
      (Math|Integer|IncrementInt (Variables|Default|GetRackNum)
        (:%20%20
          (if (not (== (Variables|Default|GetRackNum) 3))
            (CallFunction|TimerSpawn)))))))

(event Custom|TrySpawn
  (CallFunction|SpawnShop))

(event Custom|TakeShop
  (params (Ref :type BP%20Glass%20Object%20Reference))
  (bind _glassarray (Variables|Default|GetGlassArray))
  (Math|Integer|DecrementInt (Variables|Default|GetRackNum)
    (:%20%20
      (Variables|Default|SetIndexTest (Utilities|Array|FindItem _glassarray Ref))
      (Utilities|Array|RemoveItem _glassarray Ref)
      (Utilities|FlowControl|Sequence
        (:then_0
          (Utilities|Array|Clear (Variables|Default|GetStartLoc))
          (for _array_element _glassarray
            (Utilities|Array|Add (Variables|Default|GetStartLoc) (Transformation|GetActorLocation _array_element))))
        (:then_1
          (bind (_direction _alpha _angle) (Timeline|Timeline_0 PlayFromStart)
            (:Update
              (for _index (range (Variables|Default|GetIndexTest) (- (Utilities|Array|Length (Variables|Default|GetGlassArray)) 1))
                (Transformation|SetActorLocation (Utilities|Array|Get(acopy) (Variables|Default|GetGlassArray) _index) (Math|Vector|Lerp(Vector) (Utilities|Array|Get(acopy) (Variables|Default|GetStartLoc) _index) (Utilities|Select :Index _index :Option%200 (Transformation|GetWorldLocation (Variables|Default|GetSpawnPoint1)) :Option%201 (Transformation|GetWorldLocation (Variables|Default|GetSpawnPoint2)) :Option%202 (Transformation|GetWorldLocation (Variables|Default|GetSpawnPoint3))) _alpha) false false)
                (Transformation|SetActorRotation (Utilities|Array|Get(acopy) (Variables|Default|GetGlassArray) _index) (Math|Rotator|MakeRotfromZX (Math|Vector|RotateVectorAroundAxis "0.000000,0.000000,1.000000" (* _angle 1e+01) (Transformation|GetActorRightVector)) (Transformation|GetActorForwardVector (Utilities|Array|Get(acopy) (Variables|Default|GetGlassArray) _index))))))
            (:Finished
              (CallFunction|TimerSpawn))))))))

(event Custom|TimerSpawn
  (Utilities|Time|SetTimerbyEvent (delegate Custom|TrySpawn) 1e+01))

(event EventBeginPlay
  (bind _returnvalue (Game|SpawnActorfromClass "/Game/Blueprint/BP_Glass.BP_Glass_C" (Math|Transform|MakeTransform (Transformation|GetWorldLocation (Variables|Default|GetSpawnPoint)) "0, 0, 0" "1.000000,1.000000,1.000000") "AlwaysSpawn" "MultiplyWithRoot" 0 0))
  (Collision|SetActorEnableCollision _returnvalue false)
  (Utilities|Array|AddUnique (Variables|Default|GetGlassArray) _returnvalue)
  (Variables|/Game/Blueprint/BP_Glass.BP_Glass_C|SetSpawnerRef _returnvalue self)
  (bind (_direction _alpha _angle) (Timeline|Timeline PlayFromStart)
    (:Update
      (Transformation|SetActorLocation _returnvalue (Math|Vector|Lerp(Vector) (Transformation|GetWorldLocation (Variables|Default|GetSpawnPoint)) (Utilities|Select :Index (Variables|Default|GetRackNum) :Option%200 (Transformation|GetWorldLocation (Variables|Default|GetSpawnPoint1)) :Option%201 (Transformation|GetWorldLocation (Variables|Default|GetSpawnPoint2)) :Option%202 (Transformation|GetWorldLocation (Variables|Default|GetSpawnPoint3))) _alpha) false false)
      (Transformation|SetActorRotation _returnvalue (Math|Rotator|MakeRotfromZX (Math|Vector|RotateVectorAroundAxis "0.000000,0.000000,1.000000" (* _angle 2e+01) (Transformation|GetActorRightVector)) (Transformation|GetActorForwardVector _returnvalue))))
    (:Finished
      (Collision|SetActorEnableCollision _returnvalue true)
      (Math|Integer|IncrementInt (Variables|Default|GetRackNum)
        (:%20%20
          (if (not (== (Variables|Default|GetRackNum) 3))
            (CallFunction|TimerSpawn)))))))

(fn ConstructionScript)