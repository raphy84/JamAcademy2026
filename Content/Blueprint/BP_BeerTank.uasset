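; BP_BeerTank is a beer tank that refills itself over time and shows its level with a cylinder mesh.
; A Timeline restarts itself on each finish as a repeating timer, raising the target fill by a fixed step up to the maximum.
; Tick moves the normalized fill toward that target at constant speed, scaling the cylinder's height and offsetting its Z position in proportion.
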(event EventTick
  (params (DeltaSeconds :type Float%20%28single-precision%29))
  (bind _cylinder (Variables|Default|GetCylinder))
  (bind _output_get (Variables|Default|SetCurrentFill (Math|Interpolation|FInterptoConstant (Variables|Default|GetCurrentFill) (/ (Variables|Default|GetTargetFill) (Variables|Default|GetMaxFill)) DeltaSeconds 0.25)))
  (Transformation|SetRelativeScale3D _cylinder (Math|Vector|MakeVector 1.0 1.0 _output_get))
  (Transformation|SetRelativeLocation _cylinder (Math|Vector|MakeVector 0.0 0.0 (* _output_get 5e+01)) false false))

(event EventBeginPlay
  (Timeline|Timeline PlayFromStart
    (:Finished
      (Variables|Default|SetTargetFill (Math|Float|Clamp(Float) (+ (Variables|Default|GetTargetFill) 1e+01) 0.0 (Variables|Default|GetMaxFill)))
      (Timeline|Timeline PlayFromStart))))

(fn ConstructionScript)