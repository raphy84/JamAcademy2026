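; BP_Glass is a glass pickup the first-person player can hold, with a dynamic material instance on its plane.
; While not held, it rotates each tick to face the player's camera.
; Interacting plays a Timeline that lerps it to the player's GlassAnchor and attaches it, calling the spawner's TakeShop if no glass was held.
; An already held glass swaps into the new one's place by reversing that Timeline, then detaching.
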(event Custom|Swap
  (params (NewParam :type Transform))
  (bind _playerref (Variables|Default|GetPlayerRef))
  (bind _glassanchor (Variables|/Game/FirstPerson/Blueprints/BP_FirstPersonCharacter.BP_FirstPersonCharacter_C|GetGlassAnchor _playerref))
  (Variables|Default|SetIsHeld false)
  (Variables|Default|SetStartTransform NewParam)
  (Collision|SetActorEnableCollision false)
  (bind (_direction _alpha) (Timeline|Timeline ReverseFromEnd)
    (:Update
      (Transformation|SetActorTransform (Math|Transform|Lerp(Transform) (Variables|Default|GetStartTransform) (Transformation|GetWorldTransform _glassanchor) _alpha)))
    (:Finished
      (Collision|SetActorEnableCollision true)
      (switch Utilities|FlowControl|Switch|SwitchonETimelineDirection _direction
        (:Forward
          (Transformation|AttachComponentToComponent _glassanchor "None" "KeepRelative" "KeepRelative" "KeepRelative" true)
          (Transformation|SetActorRelativeTransform (Math|Transform|MakeTransform "0, 0, 0" "0, 0, 0" "1.000000,1.000000,1.000000") false false))
        (:Backward
          (Transformation|DetachFromActor "KeepWorld" "KeepWorld" "KeepWorld"))))))

(event EventBeginPlay
  (bind _asbp_first_person_character (Utilities|Casting|CastToBP_FirstPersonCharacter (Game|Player|GetPlayerPawn 0)))
  (Variables|Default|SetPlayerRef _asbp_first_person_character)
  (bind _returnvalue (Rendering|Material|CreateDynamicMaterialInstance (Variables|Default|GetMaterialParent) "None" "None" :!class /Script/Engine.KismetMaterialLibrary))
  (bind _output_get (Variables|Default|SetDMI_Glass _returnvalue))
  (Rendering|Material|SetMaterial (Variables|Default|GetPlane) 0 _output_get))

(event EventTick
  (params (DeltaSeconds :type Float%20%28single-precision%29))
  (if (not (Variables|Default|GetIsHeld))
    (Transformation|SetActorRotation (Math|Rotator|MakeRotfromZX (Math|Vector|MakeVector 0.0 0.0 1.0) (Math|Vector|Normalize (- (Transformation|GetWorldLocation (Variables|/Game/FirstPerson/Blueprints/BP_FirstPersonCharacter.BP_FirstPersonCharacter_C|GetFirstPersonCamera (Variables|Default|GetPlayerRef))) (Transformation|GetActorLocation)))))))

(event EventInteract
  (params (LazyRef :type BP%20First%20Person%20Character%20Object%20Reference))
  (bind _returnvalue (Transformation|GetActorTransform))
  (bind _playerref (Variables|Default|GetPlayerRef))
  (bind _glassanchor (Variables|/Game/FirstPerson/Blueprints/BP_FirstPersonCharacter.BP_FirstPersonCharacter_C|GetGlassAnchor _playerref))
  (bind _heldglass (Variables|/Game/FirstPerson/Blueprints/BP_FirstPersonCharacter.BP_FirstPersonCharacter_C|GetHeldGlass LazyRef)
    (:then
      (CallFunction|Swap _heldglass _returnvalue))
    (:else
      (Default|TakeShop (Variables|Default|GetSpawnerRef))))
  (Variables|/Game/FirstPerson/Blueprints/BP_FirstPersonCharacter.BP_FirstPersonCharacter_C|SetHeldGlass LazyRef self)
  (Variables|Default|SetIsHeld true)
  (Variables|Default|SetStartTransform _returnvalue)
  (Collision|SetActorEnableCollision false)
  (bind (_direction _alpha) (Timeline|Timeline PlayFromStart)
    (:Update
      (Transformation|SetActorTransform (Math|Transform|Lerp(Transform) (Variables|Default|GetStartTransform) (Transformation|GetWorldTransform _glassanchor) _alpha)))
    (:Finished
      (Collision|SetActorEnableCollision true)
      (switch Utilities|FlowControl|Switch|SwitchonETimelineDirection _direction
        (:Forward
          (Transformation|AttachComponentToComponent _glassanchor "None" "KeepRelative" "KeepRelative" "KeepRelative" true)
          (Transformation|SetActorRelativeTransform (Math|Transform|MakeTransform "0, 0, 0" "0, 0, 0" "1.000000,1.000000,1.000000") false false))
        (:Backward
          (Transformation|DetachFromActor "KeepWorld" "KeepWorld" "KeepWorld"))))))

(fn ConstructionScript)