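; BP_Fishcarte is a card actor that, when hit by a drink, acts as a menu button or an upgrade pick.
; It scales in on spawn, faces the player camera every tick and shows text through a widget.
; DrinkHit animates a hit material, then calls MenuManager, quits, or notifies ChoiceManager and applies regular upgrades to GameInstance or player stats.
; Epic cards set a Gold material parameter, but their upgrade switch is empty.
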(event Custom|Bye%20bye
  (bind (_direction _alpha) (Timeline|Spawn ReverseFromEnd)
    (:Update
      (Transformation|SetActorScale3D (Math|Vector|MakeVector _alpha _alpha _alpha)))
    (:Finished
      (switch Utilities|FlowControl|Switch|SwitchonETimelineDirection _direction
        (:Backward
          (Actor|DestroyActor))))))

(event EventBeginPlay
  (Utilities|FlowControl|Sequence
    (:then_0
      (bind _asbp_game_instance (Utilities|Casting|CastToBP_GameInstance (Game|GetGameInstance)))
      (Variables|Default|SetInstance _asbp_game_instance))
    (:then_1
      (bind _asbp_first_person_character (Utilities|Casting|CastToBP_FirstPersonCharacter (Game|Player|GetPlayerPawn 0)))
      (Variables|Default|SetPlayerRef _asbp_first_person_character)
      (bind _returnvalue (Rendering|Material|CreateDynamicMaterialInstance (Variables|Default|GetIdle) "None" "None" :!class /Script/Engine.KismetMaterialLibrary))
      (bind _output_get (Variables|Default|SetDMI_Idle _returnvalue))
      (Rendering|Material|SetScalarParameterValue _output_get "Gold" (Math|Conversions|ToFloat(Boolean) (Variables|Default|GetIsEpic)) :!class /Script/Engine.MaterialInstanceDynamic)
      (Rendering|Material|SetMaterial (Variables|Default|GetPlane) 0 (Variables|Default|GetDMI_Idle))
      (bind _returnvalue_2 (UserInterface|CreateWidget "/Game/Widgets/WBP_Fishcarte.WBP_Fishcarte_C" 0 (Variables|Default|GetText)))
      (UserInterface|SetWidget (Variables|Default|GetWidget) _returnvalue_2)
      (bind (_direction _alpha) (Timeline|Spawn PlayFromStart)
        (:Update
          (Transformation|SetActorScale3D (Math|Vector|MakeVector _alpha _alpha _alpha)))
        (:Finished
          (switch Utilities|FlowControl|Switch|SwitchonETimelineDirection _direction
            (:Backward
              (Actor|DestroyActor))))))))

(event EventDrinkHit
  (params (Drink :type DrinkEnum%20Enum :default "NewEnumerator0") (Fill :type Float%20%28double-precision%29) (IsRainbow :type Boolean))
  (bind _playerref (Variables|Default|GetPlayerRef))
  (bind _menumanager (Variables|Default|GetMenuManager))
  (bind _instance (Variables|Default|GetInstance))
  (bind _charactermovement (Variables|/Script/Engine.Character|GetCharacterMovement _playerref))
  (bind _firstpersoncamera (Variables|/Game/FirstPerson/Blueprints/BP_FirstPersonCharacter.BP_FirstPersonCharacter_C|GetFirstPersonCamera _playerref))
  (bind _returnvalue (Rendering|Material|CreateDynamicMaterialInstance (Variables|Default|GetHit) "None" "None" :!class /Script/Engine.KismetMaterialLibrary))
  (bind _output_get (Variables|Default|SetDMI_Hit _returnvalue))
  (Rendering|Material|SetScalarParameterValue _output_get "Gold" (Math|Conversions|ToFloat(Boolean) (Variables|Default|GetIsEpic)) :!class /Script/Engine.MaterialInstanceDynamic)
  (Rendering|Material|SetMaterial (Variables|Default|GetPlane) 0 _output_get)
  (Development|SetHiddeninGame (Variables|Default|GetWidget) true false)
  (bind _alpha (Timeline|Timeline PlayFromStart)
    (:Update
      (Rendering|Material|SetScalarParameterValue (Variables|Default|GetDMI_Hit) "Percent" (Math|Float|Lerp 1.0 0.0 _alpha) :!class /Script/Engine.MaterialInstanceDynamic))
    (:Finished
      (Utilities|FlowControl|Sequence
        (:then_0
          (switch Utilities|FlowControl|Switch|SwitchonFishcarteEnum (Variables|Default|GetFishcarte)
            (:NewEnumerator0
              (Default|Play (Variables|Default|GetMenuManager)))
            (:NewEnumerator1
              (Game|QuitGame 0 "Quit" false))
            (:NewEnumerator2
              (Default|LoadCredits _menumanager))
            (:NewEnumerator3
              (Default|Destroyed (Variables|Default|GetChoiceManager) self)
              (if (Variables|Default|GetIsEpic)
                (Variables|Default|SetEpicUpgrades (Variables|Default|GetEpicUpgrades))
                (switch Utilities|FlowControl|Switch|SwitchonEpicUpgrades (Variables|Default|GetEpicUpgrades))
                (else
                  (switch Utilities|FlowControl|Switch|SwitchonUpgrades (Variables|Default|GetUpgrade)
                    (:NewEnumerator0
                      (Variables|/Game/FirstPerson/Blueprints/BP_GameInstance.BP_GameInstance_C|SetGlassMultiplier _instance (* (Variables|/Game/FirstPerson/Blueprints/BP_GameInstance.BP_GameInstance_C|GetGlassMultiplier _instance) 0.75)))
                    (:NewEnumerator1
                      (Variables|/Game/FirstPerson/Blueprints/BP_GameInstance.BP_GameInstance_C|SetBeerRefillMult _instance (* (Variables|/Game/FirstPerson/Blueprints/BP_GameInstance.BP_GameInstance_C|GetBeerRefillMult _instance) 0.75)))
                    (:NewEnumerator2
                      (Variables|/Game/FirstPerson/Blueprints/BP_GameInstance.BP_GameInstance_C|SetBlueStockBoost _instance (+ (Variables|/Game/FirstPerson/Blueprints/BP_GameInstance.BP_GameInstance_C|GetBlueStockBoost _instance) 3e+01)))
                    (:NewEnumerator3
                      (Variables|/Game/FirstPerson/Blueprints/BP_GameInstance.BP_GameInstance_C|SetRedStockBoost _instance (+ (Variables|/Game/FirstPerson/Blueprints/BP_GameInstance.BP_GameInstance_C|GetRedStockBoost _instance) 3e+01)))
                    (:NewEnumerator4
                      (Variables|/Game/FirstPerson/Blueprints/BP_GameInstance.BP_GameInstance_C|SetYellowStockBoost _instance (+ (Variables|/Game/FirstPerson/Blueprints/BP_GameInstance.BP_GameInstance_C|GetYellowStockBoost _instance) 3e+01)))
                    (:NewEnumerator5
                      (Variables|/Game/FirstPerson/Blueprints/BP_GameInstance.BP_GameInstance_C|SetThrowMultiplier _instance (* (Variables|/Game/FirstPerson/Blueprints/BP_GameInstance.BP_GameInstance_C|GetThrowMultiplier _instance) 0.75)))
                    (:NewEnumerator6
                      (Camera|SetFieldOfView _firstpersoncamera (Math|Float|Min(Float) (* (Variables|/Script/Engine.CameraComponent|GetFieldOfView _firstpersoncamera) 1.05) 1.2e+02))
                      (Variables|/Script/Engine.CharacterMovementComponent|SetMaxWalkSpeed _charactermovement (+ (Variables|/Script/Engine.CharacterMovementComponent|GetMaxWalkSpeed _charactermovement) 1e+02)))
                    (:NewEnumerator7
                      (Variables|/Game/FirstPerson/Blueprints/BP_GameInstance.BP_GameInstance_C|SetRangeBoost _instance (+ (Variables|/Game/FirstPerson/Blueprints/BP_GameInstance.BP_GameInstance_C|GetRangeBoost _instance) 25.0)))
                    (:NewEnumerator9
                      (Variables|/Game/FirstPerson/Blueprints/BP_GameInstance.BP_GameInstance_C|SetGrabBoost _instance (+ (Variables|/Game/FirstPerson/Blueprints/BP_GameInstance.BP_GameInstance_C|GetGrabBoost _instance) 1e+02)))))))
            (:NewEnumerator4
              (Default|Return _menumanager))))
        (:then_1
          (Actor|DestroyActor))))))

(event EventTick
  (params (DeltaSeconds :type Float%20%28single-precision%29))
  (Transformation|SetActorRotation (Math|Rotator|MakeRotfromZX (Transformation|GetActorUpVector) (Math|Vector|Normalize (- (Transformation|GetWorldLocation (Variables|/Game/FirstPerson/Blueprints/BP_FirstPersonCharacter.BP_FirstPersonCharacter_C|GetFirstPersonCamera (Variables|Default|GetPlayerRef))) (Transformation|GetActorLocation))))))

(fn ConstructionScript)