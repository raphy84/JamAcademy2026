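; BP_GlassProjectile is a glass of colored drink that shatters on overlap and delivers its drink color and fill to targets in range.
; A dynamic material shows fill and color on a plane that billboards toward the player camera each tick.
; Overlap triggers a one-time splash, sounds and delayed destroy.
; It also widens the sphere by RangeBoost, messages overlapping enemies and one BP_Fishcarte, then disables collision next tick.
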(event OnComponentBeginOverlap(Sphere)
  (params (OverlappedComponent :type Primitive%20Component%20Object%20Reference) (OtherActor :type Actor%20Object%20Reference) (OtherComp :type Primitive%20Component%20Object%20Reference) (OtherBodyIndex :type Integer) (bFromSweep :type Boolean) (SweepResult :type Hit%20Result%20Structure%20%28by%20ref%29))
  (bind _color (Variables|Default|GetColor))
  (bind _sphere (Variables|Default|GetSphere))
  (bind _overlappingactors (Collision|GetOverlappingActors _sphere "/Game/Enemy/BP_Enemy.BP_Enemy_C" :!class /Script/Engine.PrimitiveComponent))
  (bind _returnvalue (Utilities|Select :Index _color :NewEnumerator0 "(R=1.000000,G=0.000000,B=0.000000,A=1.000000)" :NewEnumerator1 "(R=0.000000,G=1.000000,B=0.000000,A=1.000000)" :NewEnumerator2 "(R=0.000000,G=0.000000,B=1.000000,A=1.000000)" :NewEnumerator3 "(R=1.000000,G=0.500000,B=0.000000,A=1.000000)" :NewEnumerator4 "(R=1.000000,G=0.000000,B=1.000000,A=1.000000)" :NewEnumerator5 "(R=1.000000,G=1.000000,B=0.000000,A=1.000000)" :NewEnumerator6 ""))
  (Utilities|FlowControl|Sequence
    (:then_0
      (Utilities|FlowControl|DoOnce false
        (:Completed
          (Components|Activation|Deactivate (Variables|Default|GetNiagara))
          (bind _returnvalue_2 (Niagara|SpawnSystematLocation "/Game/VFX/NS_Splash.NS_Splash" (.Location (Collision|BreakHitResult SweepResult))))
          (Niagara|SetNiagaraVariable(LinearColor) _returnvalue_2 "BeerColor" (Utilities|Struct|MakeLinearColor (.r _returnvalue) (.g _returnvalue) (.b _returnvalue) (Variables|Default|GetFill)))
          (Utilities|FlowControl|Sequence
            (:then_0
              (Utilities|FlowControl|Delay 2.0)
              (Actor|DestroyActor))
            (:then_1
              (if (== (Variables|Default|GetFill) 0.0)
                _
                (else
                  (Audio|PlaySoundatLocation "/Game/Sound/SoundCue/C_Splash.C_Splash" (Transformation|GetActorLocation) "0, 0, 0" 1.0 1.0 0.0 0 0 0 0)))
              (Audio|PlaySoundatLocation "/Game/Sound/SoundCue/C_BreackGlass.C_BreackGlass" (Transformation|GetActorLocation) "0, 0, 0" 1.0 1.0 0.0 0 0 0 0))))))
    (:then_1
      (Components|Sphere|SetSphereRadius _sphere (+ (Variables|/Game/FirstPerson/Blueprints/BP_GameInstance.BP_GameInstance_C|GetRangeBoost (Variables|Default|GetAs%20BP%20Game%20Instance)) 1.5e+02) true)
      (Development|PrintString (Utilities|String|ToString(Integer) (Utilities|Array|Length _overlappingactors)))
      (for _array_element _overlappingactors
        (Class|BPIDrinks|DrinkHit(Message) _array_element (Variables|Default|GetColor) (Variables|Default|GetFill)))
      (bind _array_element_2 (Utilities|Array|ForEachLoopwithBreak (Collision|GetOverlappingActors _sphere "/Game/Blueprint/BP_Fishcarte.BP_Fishcarte_C" :!class /Script/Engine.PrimitiveComponent) :!label _label)
        (:LoopBody
          (Class|BPIDrinks|DrinkHit(Message) _array_element_2 (Variables|Default|GetColor) (Variables|Default|GetFill))
          (Audio|PlaySoundatLocation "/Game/Sound/SoundCue/C_GainAugmente.C_GainAugmente" (Transformation|GetActorLocation _array_element_2) "0, 0, 0" 0.5 1.5 0.0 0 0 0 0)
          (goto _label Break))
        (:Completed
          (Utilities|FlowControl|DelayUntilNextTick)
          (Collision|SetActorEnableCollision false))))))

(event EventBeginPlay
  (Utilities|FlowControl|Sequence
    (:then_0
      (bind _asbp_first_person_character (Utilities|Casting|CastToBP_FirstPersonCharacter (Game|Player|GetPlayerPawn 0)))
      (Variables|Default|SetPlayerRef _asbp_first_person_character)
      (bind _returnvalue (Rendering|Material|CreateDynamicMaterialInstance (.Value (Utilities|Map|Find (Variables|Default|GetMaterialParentMap) (Variables|Default|GetMaterialParent))) "None" "None" :!class /Script/Engine.KismetMaterialLibrary))
      (bind _output_get (Variables|Default|SetDMI_Glass _returnvalue))
      (Rendering|Material|SetMaterial (Variables|Default|GetPlane) 0 _output_get)
      (Rendering|Material|SetScalarParameterValue _output_get "Percent" (Variables|Default|GetFill) :!class /Script/Engine.MaterialInstanceDynamic)
      (Rendering|Material|SetVectorParameterValue _output_get "BeerColor" (Utilities|Select :Index (Variables|Default|GetColor) :NewEnumerator0 "(R=1.000000,G=0.000000,B=0.000000,A=1.000000)" :NewEnumerator1 "(R=0.000000,G=1.000000,B=0.000000,A=1.000000)" :NewEnumerator2 "(R=0.000000,G=0.000000,B=1.000000,A=1.000000)" :NewEnumerator3 "(R=1.000000,G=0.500000,B=0.000000,A=1.000000)" :NewEnumerator4 "(R=1.000000,G=0.000000,B=1.000000,A=1.000000)" :NewEnumerator5 "(R=1.000000,G=1.000000,B=0.000000,A=1.000000)" :NewEnumerator6 "") :!class /Script/Engine.MaterialInstanceDynamic))
    (:then_1
      (bind _asbp_game_instance (Utilities|Casting|CastToBP_GameInstance (Game|GetGameInstance)))
      (Variables|Default|SetAs%20BP%20Game%20Instance _asbp_game_instance))))

(event EventTick
  (params (DeltaSeconds :type Float%20%28single-precision%29))
  (Transformation|SetWorldRotation (Variables|Default|GetPlane) (Class|KismetMathLibrary|MakeRotfromYZ (Math|Vector|MakeVector 0.0 0.0 -1.0) (Math|Vector|Normalize (- (Transformation|GetWorldLocation (Variables|/Game/FirstPerson/Blueprints/BP_FirstPersonCharacter.BP_FirstPersonCharacter_C|GetFirstPersonCamera (Variables|Default|GetPlayerRef))) (Transformation|GetActorLocation)))) false false))

(fn ConstructionScript)