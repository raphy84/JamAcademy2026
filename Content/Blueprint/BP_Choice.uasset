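; Upgrade-choice manager that offers three fish cards whenever the game mode signals the end of a wave.
; A self-re-entering DoN with a delay spawns BP_Fishcarte actors one by one at Left, Mid and Right, each with a random upgrade.
; When the wave index is a multiple of five, the middle card is epic, currently only Lucky Beer.
; Destroyed dismisses the remaining cards and starts the next wave.
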(event Custom|Destroyed
  (params (NewItem :type BP%20Fishcarte%20Object%20Reference%20%28by%20ref%29))
  (bind _buttons (Variables|Default|GetButtons))
  (Utilities|Array|RemoveItem _buttons NewItem)
  (for _array_element _buttons
    (Utilities|IsValid _array_element
      (:Is%20Valid
        (Default|ByeBye _array_element))))
  (Default|CallStartWaving (Variables|Default|GetAs%20BP%20First%20Person%20Game%20Mode))
  (Audio|PlaySoundatLocation "/Game/Sound/SoundCue/C_GainAugmente.C_GainAugmente" (Transformation|GetActorLocation) "0, 0, 0" 1.0 1.0 0.0 0 0 0 0))

(event Custom|LoadChoice
  (Audio|PlaySoundatLocation "/Game/Sound/SoundWave/GainAugmente/W_MusicAugmente.W_MusicAugmente" (Transformation|GetActorLocation) "0, 0, 0" 1.0 1.0 0.0 0 0 0 0)
  (Utilities|FlowControl|Sequence
    (:then_0
      (goto _label Reset))
    (:then_1
      (bind _counter (Utilities|FlowControl|DoN 3 :!label _label)
        (:Exit
          (bind _output_get (Variables|Default|SetChosenUpgrade (.OutItem (Utilities|Array|Random (Utilities|Array|MakeArray "NewEnumerator0" "NewEnumerator1" "NewEnumerator2" "NewEnumerator3" "NewEnumerator4" "NewEnumerator5" "NewEnumerator7" "NewEnumerator6" "NewEnumerator9")))))
          (bind _output_get_2 (Variables|Default|SetChosenEpicUpgrade (.OutItem (Utilities|Array|Random (Utilities|Array|MakeArray "NewEnumerator2")))))
          (bind _returnvalue (Game|SpawnActorfromClass "/Game/Blueprint/BP_Fishcarte.BP_Fishcarte_C" (Transformation|GetWorldTransform (Utilities|Array|Get(acopy) (Utilities|Array|MakeArray (Variables|Default|GetLeft) (Variables|Default|GetMid) (Variables|Default|GetRight)) (- _counter 1))) "Undefined" "MultiplyWithRoot" 0 (Utilities|Select :Index (- _counter 1) :Option%200 "/Game/AG/UI/MI_Fish1.MI_Fish1" :Option%201 "/Game/AG/UI/MI_Fish2.MI_Fish2" :Option%202 "/Game/AG/UI/MI_Fish3.MI_Fish3") (Utilities|Select :Index (- _counter 1) :Option%200 "/Game/AG/UI/MI_Fish4.MI_Fish4" :Option%201 "/Game/AG/UI/MI_Fish5.MI_Fish5" :Option%202 "/Game/AG/UI/MI_Fish6.MI_Fish6") (Utilities|String|SelectText (Utilities|Select :Index _output_get_2 :NewEnumerator3 "" :NewEnumerator0 "Plankton" :NewEnumerator1 "Leech" :NewEnumerator2 "Lucky Beer") (Utilities|Select :Index _output_get :NewEnumerator0 "-10% Glass 
Cooldown" :NewEnumerator1 "10% Faster 
Beer Refill" :NewEnumerator2 "+20 Blue 
Storage" :NewEnumerator3 "+20 Red 
Storage" :NewEnumerator4 "+20 Yellow 
Storage" :NewEnumerator5 "10% Faster 
Throw" :NewEnumerator6 "Increased 
Move Speed" :NewEnumerator7 "+10% Beer 
Area of effect" :NewEnumerator8 "" :NewEnumerator9 "+25% Grab 
Extent") (and (== (Math|Integer|%(Integer) (Variables|/Game/Enemy/WaveManager.WaveManager_C|GetCurrentWaveIndex (Variables|/Game/FirstPerson/Blueprints/BP_FirstPersonGameMode.BP_FirstPersonGameMode_C|GetWaveManager (stale EventBeginPlay _output_get))) 5) 0) (== (- _counter 1) 1))) "NewEnumerator3" 0 _output_get self (and (== (Math|Integer|%(Integer) (Variables|/Game/Enemy/WaveManager.WaveManager_C|GetCurrentWaveIndex (Variables|/Game/FirstPerson/Blueprints/BP_FirstPersonGameMode.BP_FirstPersonGameMode_C|GetWaveManager (stale EventBeginPlay _output_get))) 5) 0) (== (- _counter 1) 1)) _output_get_2 0))
          (Utilities|Array|Add (Variables|Default|GetButtons) _returnvalue)
          (Utilities|FlowControl|Delay 0.5)
          (goto _label))))))

(event EventBeginPlay
  (bind _asbp_first_person_game_mode (Utilities|Casting|CastToBP_FirstPersonGameMode (Game|GetGameMode)))
  (bind _output_get (Variables|Default|SetAs%20BP%20First%20Person%20Game%20Mode _asbp_first_person_game_mode))
  (EventDispatchers|BindEventtoEndWave _output_get (delegate Custom|LoadChoice)))

(fn ConstructionScript)