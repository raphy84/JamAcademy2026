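; Beer tap actor that pours half a glass of its colored beer into the interacting player's held glass.
; Interact checks the glass and linked BeerTank, draws down the tank, then picks a mixed color from the tap and glass colors via nested Selects.
; A Timeline swings the lever and lerps the glass material's fill, color and rainbow, then commits them to the glass.
; An epic upgrade adds a small random chance of rainbow beer.
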(event EventBeginPlay
  (Variables|/Game/Blueprint/BP_BeerTank.BP_BeerTank_C|SetColor (Variables|Default|GetBeerTank) (Variables|Default|GetColor))
  (bind _asbp_game_instance (Utilities|Casting|CastToBP_GameInstance (Game|GetGameInstance)))
  (Variables|Default|SetAs%20BP%20Game%20Instance _asbp_game_instance))

(event Collision|EventActorBeginOverlap
  (params (OtherActor :type Actor%20Object%20Reference)))

(event EventTick
  (params (DeltaSeconds :type Float%20%28single-precision%29)))

(event EventInteract
  (params (LazyRef :type BP%20First%20Person%20Character%20Object%20Reference))
  (bind _beertank (Variables|Default|GetBeerTank))
  (bind _heldglass (Variables|/Game/FirstPerson/Blueprints/BP_FirstPersonCharacter.BP_FirstPersonCharacter_C|GetHeldGlass LazyRef)
    (:then
      (if (< (Variables|/Game/Blueprint/BP_Glass.BP_Glass_C|GetFill _heldglass) 1.0)
        (if (not (Variables|/Game/Blueprint/BP_Glass.BP_Glass_C|GetIsFilled _heldglass))
          (if (>= (Variables|/Game/Blueprint/BP_BeerTank.BP_BeerTank_C|GetTargetFill _beertank) 33.0)
            (Audio|PlaySoundatLocation "/Game/Sound/SoundCue/C_Lever.C_Lever" (Transformation|GetActorLocation) "0, 0, 0" 2.0 1.0 0.0 0 0 0 0)
            (Audio|PlaySound2D "/Game/Sound/SoundCue/C_RefilBeer.C_RefilBeer" 1.0 1.0 0.0 0 0)
            (Variables|/Game/Blueprint/BP_BeerTank.BP_BeerTank_C|SetTargetFill _beertank (- (Variables|/Game/Blueprint/BP_BeerTank.BP_BeerTank_C|GetTargetFill _beertank) 33.0))
            (Variables|/Game/Blueprint/BP_Glass.BP_Glass_C|SetIsFilled _heldglass true)
            (bind _output_get (Variables|Default|SetStartFill (Variables|/Game/Blueprint/BP_Glass.BP_Glass_C|GetFill _heldglass)))
            (bind _output_get_2 (Variables|Default|SetTargetFill (Math|Float|Clamp(Float) (+ (Variables|/Game/Blueprint/BP_Glass.BP_Glass_C|GetFill _heldglass) 0.5))))
            (bind _output_get_3 (Variables|Default|SetStartColor (Variables|/Game/Blueprint/BP_Glass.BP_Glass_C|GetColor _heldglass)))
            (Development|PrintString (Utilities|String|EnumtoString _output_get_3))
            (bind _output_get_4 (Variables|Default|SetTargetColor (Utilities|Select :Index (Variables|Default|GetColor) :NewEnumerator0 (Utilities|Select :Index (Variables|Default|GetStartColor) :NewEnumerator0 "NewEnumerator0" :NewEnumerator1 "NewEnumerator5" :NewEnumerator2 "NewEnumerator4" :NewEnumerator3 "NewEnumerator0" :NewEnumerator4 "NewEnumerator0" :NewEnumerator5 "NewEnumerator3" :NewEnumerator6 "NewEnumerator0") :NewEnumerator1 "NewEnumerator0" :NewEnumerator2 (Utilities|Select :Index (Variables|Default|GetStartColor) :NewEnumerator0 "NewEnumerator4" :NewEnumerator1 "NewEnumerator2" :NewEnumerator2 "NewEnumerator2" :NewEnumerator3 "NewEnumerator4" :NewEnumerator4 "NewEnumerator2" :NewEnumerator5 "NewEnumerator1" :NewEnumerator6 "NewEnumerator2") :NewEnumerator3 "NewEnumerator0" :NewEnumerator4 "NewEnumerator0" :NewEnumerator5 (Utilities|Select :Index (Variables|Default|GetStartColor) :NewEnumerator0 "NewEnumerator3" :NewEnumerator1 "NewEnumerator5" :NewEnumerator2 "NewEnumerator1" :NewEnumerator3 "NewEnumerator5" :NewEnumerator4 "NewEnumerator0" :NewEnumerator5 "NewEnumerator5" :NewEnumerator6 "NewEnumerator5") :NewEnumerator6 "NewEnumerator0")))
            (Utilities|FlowControl|Sequence
              (:then_0
                (if (== _output_get 0.0)
                  (Rendering|Material|SetVectorParameterValue (Variables|/Game/Blueprint/BP_Glass.BP_Glass_C|GetDMI_Glass _heldglass) "BeerColor" (Utilities|Select :Index (Variables|Default|GetColor) :NewEnumerator0 "(R=1.000000,G=0.000000,B=0.000000,A=1.000000)" :NewEnumerator1 "(R=0.000000,G=1.000000,B=0.000000,A=1.000000)" :NewEnumerator2 "(R=0.000000,G=0.000000,B=1.000000,A=1.000000)" :NewEnumerator3 "(R=1.000000,G=0.500000,B=0.000000,A=1.000000)" :NewEnumerator4 "(R=1.000000,G=0.000000,B=1.000000,A=1.000000)" :NewEnumerator5 "(R=1.000000,G=1.000000,B=0.000000,A=1.000000)" :NewEnumerator6 "") :!class /Script/Engine.MaterialInstanceDynamic)))
              (:then_1
                (Variables|Default|SetStartRainbow (Math|Conversions|ToFloat(Boolean) (Variables|/Game/Blueprint/BP_Glass.BP_Glass_C|GetIsRainbow _heldglass)))
                (bind _output_get_5 (Variables|Default|SetTargetRainbow (Math|Conversions|ToFloat(Boolean) (or (Variables|/Game/Blueprint/BP_Glass.BP_Glass_C|GetIsRainbow _heldglass) (and (Utilities|Enum|Equal(Enum) (Variables|/Game/FirstPerson/Blueprints/BP_GameInstance.BP_GameInstance_C|GetEpicUpgrade (Variables|Default|GetAs%20BP%20Game%20Instance)) "NewEnumerator2") (< (Math|Random|RandomFloat) 0.05))))))
                (bind (_direction _beer _rot) (Timeline|Timeline PlayFromStart)
                  (:Update
                    (Transformation|SetRelativeRotation (Variables|Default|GetCube1) (Math|Rotator|Lerp(Rotator) "0, 0, 0" "-90.000000,0.000000,0.000000" _rot) false false)
                    (Rendering|Material|SetScalarParameterValue (Variables|/Game/Blueprint/BP_Glass.BP_Glass_C|GetDMI_Glass _heldglass) "Percent" (Math|Float|Lerp (Variables|Default|GetStartFill) (Variables|Default|GetTargetFill) _beer) :!class /Script/Engine.MaterialInstanceDynamic)
                    (Rendering|Material|SetVectorParameterValue (Variables|/Game/Blueprint/BP_Glass.BP_Glass_C|GetDMI_Glass _heldglass) "BeerColor" (Math|Color|Lerp(LinearColor) (Utilities|Select :Index (Variables|Default|GetStartColor) :NewEnumerator0 "(R=1.000000,G=0.000000,B=0.000000,A=1.000000)" :NewEnumerator1 "(R=0.000000,G=1.000000,B=0.000000,A=1.000000)" :NewEnumerator2 "(R=0.000000,G=0.000000,B=1.000000,A=1.000000)" :NewEnumerator3 "(R=1.000000,G=0.250000,B=0.000000,A=1.000000)" :NewEnumerator4 "(R=1.000000,G=0.000000,B=1.000000,A=1.000000)" :NewEnumerator5 "(R=1.000000,G=1.000000,B=0.000000,A=1.000000)" :NewEnumerator6 "") (Utilities|Select :Index (Variables|Default|GetTargetColor) :NewEnumerator0 "(R=1.000000,G=0.000000,B=0.000000,A=1.000000)" :NewEnumerator1 "(R=0.000000,G=1.000000,B=0.000000,A=1.000000)" :NewEnumerator2 "(R=0.000000,G=0.000000,B=1.000000,A=1.000000)" :NewEnumerator3 "(R=1.000000,G=0.250000,B=0.000000,A=1.000000)" :NewEnumerator4 "(R=1.000000,G=0.000000,B=1.000000,A=1.000000)" :NewEnumerator5 "(R=1.000000,G=1.000000,B=0.000000,A=1.000000)" :NewEnumerator6 "") _beer) :!class /Script/Engine.MaterialInstanceDynamic)
                    (Rendering|Material|SetScalarParameterValue (Variables|/Game/Blueprint/BP_Glass.BP_Glass_C|GetDMI_Glass _heldglass) "Rainbow" (Math|Float|Lerp (Variables|Default|GetStartRainbow) (Variables|Default|GetTargetRainbow) _beer) :!class /Script/Engine.MaterialInstanceDynamic))
                  (:Finished
                    (Variables|/Game/Blueprint/BP_Glass.BP_Glass_C|SetIsFilled _heldglass false)
                    (Variables|/Game/Blueprint/BP_Glass.BP_Glass_C|SetFill _heldglass _output_get_2)
                    (Variables|/Game/Blueprint/BP_Glass.BP_Glass_C|SetColor _heldglass _output_get_4)
                    (Variables|/Game/Blueprint/BP_Glass.BP_Glass_C|SetIsRainbow _heldglass (== _output_get_5 1.0))))))))))
    (:else)))

(fn ConstructionScript)