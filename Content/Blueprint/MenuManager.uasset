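; MenuManager is the main menu actor, spawning BP_Fishcarte actors as Play, Credits and Quit buttons at three scene points, staggered by delays.
; Each card receives idle and hit materials, a label and a manager reference.
; LoadCredits dismisses other cards, spawns a Return card and fades in a widget-component credits screen, which Return reverses before reloading.
; Play dismisses other cards and fires the game mode's StartWaving and its own music dispatcher.
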(event Custom|LoadMenu
  (Utilities|FlowControl|Delay 0.5)
  (bind _returnvalue (Game|SpawnActorfromClass "/Game/Blueprint/BP_Fishcarte.BP_Fishcarte_C" (Transformation|GetWorldTransform (Variables|Default|GetLeft)) "Undefined" "MultiplyWithRoot" 0 "/Game/AG/UI/MI_Fish1.MI_Fish1" "/Game/AG/UI/MI_Fish4.MI_Fish4" "PLAY" "NewEnumerator0" self "NewEnumerator0" 0 0))
  (Variables|Default|SetPlayButton _returnvalue)
  (Utilities|FlowControl|Delay 0.5)
  (bind _returnvalue_2 (Game|SpawnActorfromClass "/Game/Blueprint/BP_Fishcarte.BP_Fishcarte_C" (Transformation|GetWorldTransform (Variables|Default|GetMid)) "Undefined" "MultiplyWithRoot" 0 "/Game/AG/UI/MI_Fish2.MI_Fish2" "/Game/AG/UI/MI_Fish5.MI_Fish5" "CREDITS" "NewEnumerator2" self "NewEnumerator0" 0 0))
  (Variables|Default|SetCredit _returnvalue_2)
  (Utilities|FlowControl|Delay 0.5)
  (bind _returnvalue_3 (Game|SpawnActorfromClass "/Game/Blueprint/BP_Fishcarte.BP_Fishcarte_C" (Transformation|GetWorldTransform (Variables|Default|GetRight)) "Undefined" "MultiplyWithRoot" 0 "/Game/AG/UI/MI_Fish3.MI_Fish3" "/Game/AG/UI/MI_Fish6.MI_Fish6" "QUIT" "NewEnumerator1" self "NewEnumerator0" 0 0))
  (Variables|Default|SetQuitButton _returnvalue_3))

(event Custom|LoadCredits
  (bind _credits (Variables|Default|GetCredits))
  (Default|ByeBye (Variables|Default|GetPlayButton))
  (Utilities|FlowControl|Delay 0.5)
  (Game|SpawnActorfromClass "/Game/Blueprint/BP_Fishcarte.BP_Fishcarte_C" (Transformation|GetWorldTransform (Variables|Default|GetLeft)) "Undefined" "MultiplyWithRoot" 0 "/Game/AG/UI/MI_Fish2.MI_Fish2" "/Game/AG/UI/MI_Fish5.MI_Fish5" "RETURN" "NewEnumerator4" self "NewEnumerator0" 0 0)
  (Class|UserWidget|PlayAnimationForward _credits (Variables|/Game/Widgets/WBP_Credits.WBP_Credits_C|GetFadeIn _credits) 1.0 false))

(event Custom|Return
  (bind _credits (Variables|Default|GetCredits))
  (Class|UserWidget|PlayAnimationReverse _credits (Variables|/Game/Widgets/WBP_Credits.WBP_Credits_C|GetFadeIn _credits) 1.0 false)
  (Utilities|FlowControl|Delay 0.5)
  (CallFunction|LoadMenu))

(event Custom|Play
  (Default|ByeBye (Variables|Default|GetCredit))
  (Default|CallStartWaving (Variables|Default|GetAs%20BP%20First%20Person%20Game%20Mode))
  (Default|CallLaucheMusique))

(event EventBeginPlay
  (bind _asbp_first_person_game_mode (Utilities|Casting|CastToBP_FirstPersonGameMode (Game|GetGameMode)))
  (Variables|Default|SetAs%20BP%20First%20Person%20Game%20Mode _asbp_first_person_game_mode)
  (bind _returnvalue (UserInterface|CreateWidget "/Game/Widgets/WBP_Credits.WBP_Credits_C"))
  (bind _output_get (Variables|Default|SetCredits _returnvalue))
  (UserInterface|SetWidget (Variables|Default|GetWidget) _output_get)
  (Utilities|FlowControl|Delay 0.5)
  (bind _returnvalue_2 (Game|SpawnActorfromClass "/Game/Blueprint/BP_Fishcarte.BP_Fishcarte_C" (Transformation|GetWorldTransform (Variables|Default|GetLeft)) "Undefined" "MultiplyWithRoot" 0 "/Game/AG/UI/MI_Fish1.MI_Fish1" "/Game/AG/UI/MI_Fish4.MI_Fish4" "PLAY" "NewEnumerator0" self "NewEnumerator0" 0 0))
  (Variables|Default|SetPlayButton _returnvalue_2)
  (Utilities|FlowControl|Delay 0.5)
  (bind _returnvalue_3 (Game|SpawnActorfromClass "/Game/Blueprint/BP_Fishcarte.BP_Fishcarte_C" (Transformation|GetWorldTransform (Variables|Default|GetMid)) "Undefined" "MultiplyWithRoot" 0 "/Game/AG/UI/MI_Fish2.MI_Fish2" "/Game/AG/UI/MI_Fish5.MI_Fish5" "CREDITS" "NewEnumerator2" self "NewEnumerator0" 0 0))
  (Variables|Default|SetCredit _returnvalue_3)
  (Utilities|FlowControl|Delay 0.5)
  (bind _returnvalue_4 (Game|SpawnActorfromClass "/Game/Blueprint/BP_Fishcarte.BP_Fishcarte_C" (Transformation|GetWorldTransform (Variables|Default|GetRight)) "Undefined" "MultiplyWithRoot" 0 "/Game/AG/UI/MI_Fish3.MI_Fish3" "/Game/AG/UI/MI_Fish6.MI_Fish6" "QUIT" "NewEnumerator1" self "NewEnumerator0" 0 0))
  (Variables|Default|SetQuitButton _returnvalue_4))

(fn ConstructionScript)